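; Dataprep operation that flattens actor hierarchies by attaching nested descendants directly to their "level" actors.
; It collects unique context actors whose display name contains PartOfLabel into Levels, then gathers each one's descendants with a DataprepHierarchySelectionTransform.
; Descendants whose parent label differs from the level actor's are reattached to it, keeping world location and rotation but relative scale.
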(event EventOnExecution
  (params (InContext :type Dataprep%20Context%20Structure%20%28by%20ref%29))
  (bind _returnvalue (Game|ConstructObjectfromClass "/Script/DataprepLibraries.DataprepHierarchySelectionTransform" self))
  (bind _output_get (Variables|Default|SetHierarchy _returnvalue))
  (Variables|/Script/DataprepLibraries.DataprepHierarchySelectionTransform|SetSelectionPolicy _output_get "AllDescendants")
  (Utilities|Array|Clear (Variables|Default|GetLevels))
  (for _array_element (Utilities|Struct|BreakDataprepContext InContext)
    (bind _asactor (Utilities|Casting|CastToActor _array_element))
    (if (Utilities|String|Contains (Utilities|GetDisplayName _array_element) (Variables|Default|GetPartOfLabel))
      (Utilities|Array|AddUnique (Variables|Default|GetLevels) _asactor)))
  (for _array_element_2 (Variables|Default|GetLevels)
    (Utilities|Array|Clear (Variables|Default|GetObjectsToMerge))
    (bind _outobjects (Class|DataprepSelectionTransform|Execute (Variables|Default|GetHierarchy) (Utilities|Array|MakeArray _array_element_2)))
    (for _array_element_3 _outobjects
      (bind _asactor_2 (Utilities|Casting|CastToActor _array_element_3))
      (if (Utilities|Enum|NotEqual(Enum) (Class|Actor|GetActorLabel _array_element_2) (Class|Actor|GetActorLabel (Actor|GetAttachParentActor _asactor_2)))
        (Transformation|AttachActorToActor _asactor_2 _array_element_2 "None" "KeepWorld" "KeepWorld" "KeepRelative" true)))))