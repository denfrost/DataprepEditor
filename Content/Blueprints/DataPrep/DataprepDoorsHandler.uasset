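; Dataprep operation that re-parents matching actors, apparently door parts judging by the asset name, during scene import processing.
; On execution it scans the context objects for actors whose label contains the ExcludeActorLabel substring.
; Each match with a valid parent and grandparent is attached directly to the grandparent, lifting it one level up the hierarchy with keep-relative transform rules.
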(event EventOnExecution
  (params (InContext :type Dataprep%20Context%20Structure%20%28by%20ref%29))
  (for _array_element (Utilities|Struct|BreakDataprepContext InContext)
    (bind _asactor (Utilities|Casting|CastToActor _array_element))
    (if (Utilities|String|Contains (Class|Actor|GetActorLabel _asactor) (Variables|Default|GetExclude%20Actor%20Label))
      (Utilities|IsValid (Actor|GetAttachParentActor _asactor)
        (:Is%20Valid
          (Utilities|IsValid (Actor|GetAttachParentActor (Actor|GetAttachParentActor _asactor))
            (:Is%20Valid
              (Transformation|AttachActorToActor _asactor (Actor|GetAttachParentActor (Actor|GetAttachParentActor _asactor)) "None" "KeepRelative" "KeepRelative" "KeepRelative" true))))))))