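; Dataprep operation that filters level objects by display-name label and gathers candidates for a static mesh merge, apparently as a test.
; Objects with over four Datasmith metadata entries contribute their static mesh component if plain Actors, or themselves if StaticMeshActors.
; A final pass separates StaticMeshActors from failures, which include those components, and prints diagnostics.
; The metadata filter affects only logging, and the merge call is disconnected.
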(event EventOnExecution
  (params (InContext :type Dataprep%20Context%20Structure%20%28by%20ref%29))
  (bind _filtermetadata (Variables|Default|GetFilterMetadata))
  (bind _allobjects (Variables|Default|GetAllObjects))
  (bind _staticmeshesformerge (Variables|Default|GetStaticMeshesForMerge))
  (bind _filterlabel (Variables|Default|GetFilterLabel))
  (bind _failedobjects (Variables|Default|GetFailedObjects))
  (bind _objectstomerge (Variables|Default|GetObjectsToMerge))
  (bind _returnvalue (Utilities|String|StringToName _filtermetadata))
  (Utilities|Array|Clear (Variables|Default|GetFailedObjects))
  (Utilities|Array|Clear (Variables|Default|GetStaticMeshesForMerge))
  (Utilities|Array|Clear (Variables|Default|GetObjectsToMerge))
  (Utilities|Array|Clear (Variables|Default|GetAllObjects))
  (for _array_element (Utilities|Struct|BreakDataprepContext InContext)
    (if (Utilities|String|Contains (Utilities|GetDisplayName _array_element) _filterlabel)
      (Utilities|Array|Add _allobjects _array_element :!label _label)
      (elif (Utilities|Enum|Equal(Enum) _filterlabel "")
        (goto _label))))
  (Development|PrintString _array_element (Utilities|String|ToString(Text) (Utilities|Text|FormatText "|||||======== All Objects count {count} ===========||||" (Utilities|Array|Length _allobjects))))
  (for (_array_element_2 _array_index) (Variables|Default|GetAllObjects)
    (bind _returnvalue_2 (Class|DatasmithContentBlueprintLibrary|GetDatasmithUserData _array_element_2))
    (if (> (Utilities|Map|Length (Variables|/Script/DatasmithContent.DatasmithAssetUserData|GetMetaData _returnvalue_2)) 4)
      (Development|PrintString _returnvalue_2 (Utilities|String|ToString(Text) (Utilities|Text|FormatText "[{Index}] Class {Type} MetaData count {count}" _array_index (Utilities|GetClassDisplayName (Utilities|GetClass _array_element_2)) (Utilities|Map|Length (Variables|/Script/DatasmithContent.DatasmithAssetUserData|GetMetaData _returnvalue_2)))) false false)
      (if (== (Utilities|GetClass _array_element_2) "/Script/Engine.Actor")
        (bind _asactor (Utilities|Casting|CastToActor _array_element_2))
        (Development|PrintString _asactor (Utilities|String|ToString(Text) (Utilities|Text|FormatText "Class StaticMeshComp {Name} From Actor" (Utilities|GetObjectName (Actor|GetComponentbyClass _asactor "/Script/Engine.StaticMeshComponent")))) false false)
        (Utilities|IsValid (Actor|GetComponentbyClass _asactor "/Script/Engine.StaticMeshComponent")
          (:Is%20Valid
            (Utilities|Array|Add _objectstomerge (Actor|GetComponentbyClass _asactor "/Script/Engine.StaticMeshComponent"))))
        (else
          (bind _asstatic_mesh_actor (Utilities|Casting|CastToStaticMeshActor _array_element_2))
          (Utilities|Array|Add _objectstomerge _asstatic_mesh_actor)
          (bind _keys (Utilities|Map|Keys (Variables|/Script/DatasmithContent.DatasmithAssetUserData|GetMetaData _returnvalue_2)))
          (bind _values (Utilities|Map|Values (Variables|/Script/DatasmithContent.DatasmithAssetUserData|GetMetaData _returnvalue_2)))
          (for (_array_element_3 _array_index_2) _keys
            (if (Utilities|Name|Equal(Name) _array_element_3 _returnvalue)
              (Development|PrintString _returnvalue_2 (Utilities|String|ToString(Text) (Utilities|Text|FormatText "{Key} = {Value}" (Utilities|String|ToString(Name) _array_element_3) (Utilities|Array|Get(acopy) _values _array_index_2))) false false :!label _label_2)
              (elif (Utilities|Name|Equal(Name) _returnvalue "")
                (goto _label_2))))))))
  (Development|PrintString _array_element_2 (Utilities|String|ToString(Text) (Utilities|Text|FormatText "|||||======== All Objects for MERGE count {count} ===========||||" (Utilities|Text|ToText(Integer) (Utilities|Array|Length (Variables|Default|GetObjectsToMerge))))))
  (for (_array_element_4 _array_index_3) (Variables|Default|GetObjectsToMerge)
    (Class|DatasmithContentBlueprintLibrary|GetDatasmithUserData _array_element_4)
    (Development|PrintString _array_element_4 (Utilities|String|ToString(Text) (Utilities|Text|FormatText "[{Index}] Class {Type} " _array_index_3 (Utilities|GetClassDisplayName (Utilities|GetClass _array_element_4)))) false)
    (bind _asstatic_mesh_actor_2 (Utilities|Casting|CastToStaticMeshActor _array_element_4)
      (:then
        (Utilities|Array|Add _staticmeshesformerge _asstatic_mesh_actor_2))
      (:CastFailed
        (Utilities|Array|Add (Variables|Default|GetFailedObjects) _array_element_4))))
  (Development|PrintString 0 (Utilities|String|ToString(Integer) (Utilities|Array|Length _staticmeshesformerge)))
  (Development|PrintString 0 (Utilities|String|ToString(Integer) (Utilities|Array|Length _failedobjects)))
  (for _array_element_5 _failedobjects
    (Development|PrintString 0 (Utilities|GetClassDisplayName (Utilities|GetClass _array_element_5)))))