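; Dataprep operation that replaces imported Datasmith static mesh actors with BP_POI actors, named as condos.
; Each POI copies the source's location, rotation, mesh and scale into itself and its POIVolume, then attaches to the same parent.
; Datasmith metadata supplies the TeleportPoint's relative position from door coordinates divided by ten, and the ID from building id and slug.
; The source actor is deleted afterwards.
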(event EventOnExecution
  (params (InContext :type Dataprep%20Context%20Structure%20%28by%20ref%29))
  (for (_array_element _array_index) (Utilities|Struct|BreakDataprepContext InContext)
    (bind _asstatic_mesh_actor (Utilities|Casting|CastToStaticMeshActor _array_element))
    (bind _returnvalue (Class|DataprepEditingOperation|CreateActor "/Game/Blueprints/BP_POI.BP_POI_C" (Utilities|String|Append "Condo_" (Utilities|String|ToString(Integer) _array_index))))
    (bind _asbp_poi (Utilities|Casting|CastToBP_POI _returnvalue))
    (Transformation|SetActorLocationAndRotation _returnvalue (Transformation|GetActorLocation _asstatic_mesh_actor) (Transformation|GetActorRotation _asstatic_mesh_actor))
    (Components|StaticMesh|SetStaticMesh (Variables|/Script/VEC.VECBasePOI|GetPOIVolume _asbp_poi) (Variables|/Script/Engine.StaticMeshComponent|GetStaticMesh (Variables|/Script/Engine.StaticMeshActor|GetStaticMeshComponent _asstatic_mesh_actor)))
    (Transformation|SetRelativeScale3D (Variables|/Script/VEC.VECBasePOI|GetPOIVolume _asbp_poi) (Variables|/Script/Engine.SceneComponent|GetRelativeScale3D (Variables|/Script/Engine.StaticMeshActor|GetStaticMeshComponent _asstatic_mesh_actor)))
    (Transformation|AttachActorToActor _asbp_poi (Actor|GetAttachParentActor _asstatic_mesh_actor) "None" "KeepRelative" "KeepRelative" "KeepRelative" true)
    (bind _returnvalue_2 (Class|DatasmithContentBlueprintLibrary|GetDatasmithUserData _asstatic_mesh_actor))
    (if (Math|Boolean|ANDBoolean (.ReturnValue (Utilities|Map|Find (Variables|/Script/DatasmithContent.DatasmithAssetUserData|GetMetaData _returnvalue_2) "Element_Door_X")) (.ReturnValue (Utilities|Map|Find (Variables|/Script/DatasmithContent.DatasmithAssetUserData|GetMetaData _returnvalue_2) "Element_Door_Y")) (.ReturnValue (Utilities|Map|Find (Variables|/Script/DatasmithContent.DatasmithAssetUserData|GetMetaData _returnvalue_2) "Element_Door_Z")))
      (Transformation|SetRelativeLocation (Variables|/Script/VEC.VECBasePOI|GetTeleportPoint _asbp_poi) (/ (Math|Vector|MakeVector (Math|Conversions|ToFloat(Integer) (.Value (Utilities|Map|Find (Variables|/Script/DatasmithContent.DatasmithAssetUserData|GetMetaData _returnvalue_2) "Element_Door_X"))) (Math|Conversions|ToFloat(Integer) (.Value (Utilities|Map|Find (Variables|/Script/DatasmithContent.DatasmithAssetUserData|GetMetaData _returnvalue_2) "Element_Door_Y"))) (Math|Conversions|ToFloat(Integer) (.Value (Utilities|Map|Find (Variables|/Script/DatasmithContent.DatasmithAssetUserData|GetMetaData _returnvalue_2) "Element_Door_Z")))) 1e+01) false true))
    (if (and (.ReturnValue (Utilities|Map|Find (Variables|/Script/DatasmithContent.DatasmithAssetUserData|GetMetaData _returnvalue_2) "Element_building_id")) (.ReturnValue (Utilities|Map|Find (Variables|/Script/DatasmithContent.DatasmithAssetUserData|GetMetaData _returnvalue_2) "Element_slug")))
      (Variables|/Script/VEC.VECBasePOI|SetID _asbp_poi (Utilities|String|Append (.Value (Utilities|Map|Find (Variables|/Script/DatasmithContent.DatasmithAssetUserData|GetMetaData _returnvalue_2) "Element_building_id")) "-" (.Value (Utilities|Map|Find (Variables|/Script/DatasmithContent.DatasmithAssetUserData|GetMetaData _returnvalue_2) "Element_slug")))))
    (Class|DataprepEditingOperation|DeleteObject _array_element)))