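; Dataprep operation that groups imported Datasmith actors by level metadata for per-level mesh merging.
; LevelMaker collects unique FilterMetadataKey values, then gathers actors whose hard-coded Element_Export_Level value matches each.
; Non-StaticMeshActors get StaticMeshActor copies, and those whose names match a DTReplacerActors row are replaced by that row's Blueprint class.
; If MERGALLLEVELS is set, each group merges into an asset under /Game/Level/ without spawning it.
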(event EventOnExecution
  (params (InContext :type Dataprep%20Context%20Structure%20%28by%20ref%29))
  (bind _output_get (Variables|Default|SetStart_Objects (Utilities|Struct|BreakDataprepContext InContext)))
  ;[1 1 1] ConvertsToActors and MergeSeparate For levels
  (Utilities|FlowControl|Sequence
    (:then_0
      ;[1 1 1] Gather All Objects and Filter only for Merging
      (bind _all_sma (CallFunction|LevelMaker _output_get (Utilities|Map|MakeMap (Variables|Default|GetFilterMetadata%20Key) (Variables|Default|GetFilterMetadata%20Value))))
      (Development|PrintString 0 (Utilities|String|ToString(Text) (Utilities|Text|FormatText "Finished  WORK : {All_SMA} from {AllCount} Objects |||||||||||||||" (Utilities|Array|Length _all_sma) (Utilities|Array|Length _output_get)))))))

(fn LevelMaker
  (params (In%20Array :type Array%20of%20Object%20Object%20References) (KeyValue :type Map%20of%20Names%20to%20Strings))
  (bind _dt_replaceractors (Variables|Default|GetDT_ReplacerActors))
  (bind _local_all_sma (LocalVariables|Getlocal_All_SMA))
  (bind _local_alllevelsformerge (LocalVariables|Getlocal_AllLevelsForMerge))
  (for _array_element In%20Array
    (bind _returnvalue (Class|DatasmithContentBlueprintLibrary|GetDatasmithUserData _array_element))
    (if (.ReturnValue (Utilities|Map|Find (Variables|/Script/DatasmithContent.DatasmithAssetUserData|GetMetaData _returnvalue) (Variables|Default|GetFilterMetadata%20Key)))
      (Utilities|Array|AddUnique _local_alllevelsformerge (.Value (Utilities|Map|Find (Variables|/Script/DatasmithContent.DatasmithAssetUserData|GetMetaData _returnvalue) (Variables|Default|GetFilterMetadata%20Key))))))
  (for _array_element_2 _local_alllevelsformerge
    (Utilities|Array|Clear (LocalVariables|Getlocal_All_SMA))
    (Development|PrintString 0 (Utilities|String|Append "Begin Merging " _array_element_2))
    (bind (_outobjects _outvalues) (Class|DatasmithContentBlueprintLibrary|GetAllObjectsandValuesforKey "Element_Export_Level" "/Script/Engine.Actor"))
    (for (_array_element_3 _array_index) _outobjects
      ;[0 0 0 1 56] Filter Levels
      (if (Utilities|Enum|Equal(Enum) (Utilities|Array|Get(acopy) _outvalues _array_index) _array_element_2)
        (bind _asstatic_mesh_actor (Utilities|Casting|CastToStaticMeshActor _array_element_3)
          (:then
            (Development|PrintString 0 (Utilities|String|ToString(Text) (Utilities|Text|FormatText "Index[{Index}] Class[{Class}] Element_Export_Level = [{Lev}] " _array_index (Utilities|GetClassDisplayName (Utilities|GetClass _array_element_3)) (Utilities|Array|Get(acopy) _outvalues _array_index))))
            (Utilities|Array|Add (LocalVariables|Getlocal_All_SMA) _asstatic_mesh_actor))
          (:CastFailed
            (Development|PrintString 0 (Utilities|String|ToString(Text) (Utilities|Text|FormatText "Cast Failed Index[{Index}] Class[{Class}] Element_Export_Level = [{Lev}] " _array_index (Utilities|GetClassDisplayName (Utilities|GetClass _array_element_3)) (Utilities|Array|Get(acopy) _outvalues _array_index))))
            ;[0 0 0 1 66] CONSTRUCT
            (bind _asactor (Utilities|Casting|CastToActor _array_element_3))
            (bind _returnvalue_2 (Class|DataprepEditingOperation|CreateActor "/Script/Engine.StaticMeshActor" (Utilities|GetDisplayName _array_element_3)))
            (bind _asstatic_mesh_actor_2 (Utilities|Casting|CastToStaticMeshActor _returnvalue_2))
            (Utilities|IsValid (Variables|/Script/Engine.StaticMeshComponent|GetStaticMesh (Actor|GetComponentbyClass _asactor "/Script/Engine.StaticMeshComponent"))
              (:Is%20Valid
                (Components|StaticMesh|SetStaticMesh (Variables|/Script/Engine.StaticMeshActor|GetStaticMeshComponent _asstatic_mesh_actor_2) (Variables|/Script/Engine.StaticMeshComponent|GetStaticMesh (Actor|GetComponentbyClass _asactor "/Script/Engine.StaticMeshComponent")))
                (Transformation|SetWorldTransform (Variables|/Script/Engine.StaticMeshActor|GetStaticMeshComponent _asstatic_mesh_actor_2) (Transformation|GetWorldTransform (Actor|GetComponentbyClass _asactor "/Script/Engine.StaticMeshComponent")) false false)
                (bind _asstatic_mesh_actor_3 (Utilities|Casting|CastToStaticMeshActor _returnvalue_2))
                (Utilities|Array|Add (LocalVariables|Getlocal_NewAdditional_SMA) _asstatic_mesh_actor_3)
                (Utilities|Array|Add (LocalVariables|Getlocal_All_SMA) _asstatic_mesh_actor_3)
                ;[0 0 0 1 66] filter by table
                (bind _outrownames (DataTable|GetDataTableRowNames _dt_replaceractors))
                (bind _array_element_4 (Utilities|Array|ForEachLoopwithBreak _outrownames :!label _label)
                  (:LoopBody
                    (bind _returnvalue_3 (Utilities|GetDataTableRow _dt_replaceractors _array_element_4)
                      (:then
                        (if (Utilities|String|Contains (Utilities|GetDisplayName _array_element_3) (Utilities|String|ToString(Name) (.MeshName (Utilities|Struct|BreakStruct_ReplacerActors _returnvalue_3))))
                          (Development|PrintString 0 (Utilities|String|ToString(Text) (Utilities|Text|FormatText "Equal {Meshname} by {DTMeshname} " (Utilities|GetDisplayName _array_element_3) (.MeshName (Utilities|Struct|BreakStruct_ReplacerActors _returnvalue_3)))))
                          ;[0 0 0 1 66] REPLACE
                          (bind _returnvalue_4 (Utilities|GetDataTableRow (Variables|Default|GetDT_ReplacerActors) _array_element_4)
                            (:then
                              (Development|PrintString _asactor (Utilities|String|ToString(Text) (Utilities|Text|FormatText "Replaced {New} by {Actor} " (Utilities|GetDisplayName _asactor) (Utilities|GetClassDisplayName (.BPClassForReplace (Utilities|Struct|BreakStruct_ReplacerActors _returnvalue_4))))))
                              (bind _returnvalue_5 (Class|DataprepEditingOperation|CreateActor (.BPClassForReplace (Utilities|Struct|BreakStruct_ReplacerActors _returnvalue_4)) (Utilities|GetDisplayName _asactor)))
                              (Transformation|SetActorTransform _returnvalue_5 (Transformation|GetWorldTransform (Actor|GetComponentbyClass _asactor "/Script/Engine.StaticMeshComponent")))
                              (Components|StaticMesh|SetStaticMesh (Actor|GetComponentbyClass _returnvalue_5 "/Script/Engine.StaticMeshComponent") (Variables|/Script/Engine.StaticMeshComponent|GetStaticMesh (Actor|GetComponentbyClass _asactor "/Script/Engine.StaticMeshComponent")))
                              (Actor|DestroyActor _asactor)
                              (Actor|DestroyActor _returnvalue_2)
                              (goto _label Break))))))))))))))
    ;[0 0 0 1 85] MERGE
    (if (Variables|Default|GetMERG_ALL_LEVELS)
      (Development|PrintString 0 (Utilities|String|Append "Finished Merging " _array_element_2 "  merged " (Utilities|String|ToString(Integer) (Utilities|Array|Length _local_all_sma)) " objects"))
      (Class|EditorLevelLibrary|MergeStaticMeshActors _local_all_sma (Utilities|Struct|MakeEditorScriptingMergeStaticMeshActorsOptions false (Utilities|String|Append "/Game/Level/" _array_element_2) (Utilities|Struct|MakeMeshMergingSettings 256 "(TextureSize=(X=1024,Y=1024),GutterSpace=4.000000,MetallicConstant=0.000000,RoughnessConstant=0.500000,AnisotropyConstant=0.000000,SpecularConstant=0.500000,OpacityConstant=1.000000,OpacityMaskConstant=1.000000,AmbientOcclusionConstant=1.000000,TextureSizingType=TextureSizingType_UseSingleTextureSize,MaterialMergeType=MaterialMergeType_Default,BlendMode=BLEND_Opaque,bAllowTwoSidedMaterial=True,bNormalMap=True,bTangentMap=False,bMetallicMap=False,bRoughnessMap=False,bAnisotropyMap=False,bSpecularMap=False,bEmissiveMap=False,bOpacityMap=False,bOpacityMaskMap=False,bAmbientOcclusionMap=False,DiffuseTextureSize=(X=1024,Y=1024),NormalTextureSize=(X=1024,Y=1024),TangentTextureSize=(X=1024,Y=1024),MetallicTextureSize=(X=1024,Y=1024),RoughnessTextureSize=(X=1024,Y=1024),AnisotropyTextureSize=(X=1024,Y=1024),SpecularTextureSize=(X=1024,Y=1024),EmissiveTextureSize=(X=1024,Y=1024),OpacityTextureSize=(X=1024,Y=1024),OpacityMaskTextureSize=(X=1024,Y=1024),AmbientOcclusionTextureSize=(X=1024,Y=1024))" 0 "AllLODs" false false false false false false false true false false false) false _array_element_2))))
  ;[0 0 0 1 94] Finish
  (return (LocalVariables|Getlocal_All_SMA)))