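; Test Dataprep operation that prints the display names of context objects whose names contain PartOfLabel.
; It creates an all-descendants hierarchy selection transform on execution, but the live path never runs it.
; Disconnected chains hold a per-level merge prototype: gather matching actors, select their descendants, skip labels containing "Doors_Door", and pass the rest to a merge-actors operation.
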(event EventOnExecution
  (params (InContext :type Dataprep%20Context%20Structure%20%28by%20ref%29))
  (bind _returnvalue (Game|ConstructObjectfromClass "/Script/DataprepLibraries.DataprepHierarchySelectionTransform" self))
  (bind _output_get (Variables|Default|SetHierarchy _returnvalue))
  (Variables|/Script/DataprepLibraries.DataprepHierarchySelectionTransform|SetSelectionPolicy _output_get "AllDescendants")
  (for _array_element (Utilities|Struct|BreakDataprepContext InContext)
    (if (Utilities|String|Contains (Utilities|GetDisplayName _array_element) (Variables|Default|GetPartOfLabel))
      (Development|PrintString 0 (Utilities|GetDisplayName _array_element)))))