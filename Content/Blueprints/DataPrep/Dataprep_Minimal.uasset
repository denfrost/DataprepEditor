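; A Dataprep operation Blueprint that logs the Datasmith metadata of objects whose display name contains the PartOfLabel substring.
; On execution it loops over the context's objects, prints each match's name, then its metadata count and every key-value pair from its Datasmith user data.
; An unconnected branch that would create an all-descendants hierarchy selection transform before the loop never runs.
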(event EventOnExecution
  (params (InContext :type Dataprep%20Context%20Structure%20%28by%20ref%29))
  (for _array_element (Utilities|Struct|BreakDataprepContext InContext)
    (if (Utilities|String|Contains (Utilities|GetDisplayName _array_element) (Variables|Default|GetPartOfLabel))
      (Development|PrintString _array_element (Utilities|GetDisplayName _array_element) false)
      (bind _returnvalue (Class|DatasmithContentBlueprintLibrary|GetDatasmithUserData _array_element))
      (Development|PrintString _returnvalue (Utilities|String|ToString(Text) (Utilities|Text|FormatText "[{Obj}] MetaData count {count}" (Utilities|GetDisplayName _array_element) (Utilities|Map|Length (Variables|/Script/DatasmithContent.DatasmithAssetUserData|GetMetaData _returnvalue)))))
      (bind _keys (Utilities|Map|Keys (Variables|/Script/DatasmithContent.DatasmithAssetUserData|GetMetaData _returnvalue)))
      (bind _values (Utilities|Map|Values (Variables|/Script/DatasmithContent.DatasmithAssetUserData|GetMetaData _returnvalue)))
      (for (_array_element_2 _array_index) _keys
        (Development|PrintString _returnvalue (Utilities|String|ToString(Text) (Utilities|Text|FormatText "{Key} = {Value}" (Utilities|String|ToString(Name) _array_element_2) (Utilities|Array|Get(acopy) _values _array_index))))))))