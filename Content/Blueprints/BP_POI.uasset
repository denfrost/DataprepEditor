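; BP_POI is a point-of-interest actor with a TeleportPoint component.
; Its construction script runs the parent script, then traces 1000 units straight down on the Visibility channel.
; Disconnected logic would place TeleportPoint 100 units above the hit, compensating for actor scale, so the trace result currently has no effect.
; The event graph holds no active logic.
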(event EventBeginPlay)

(fn ConstructionScript
  (bind _returnvalue (Transformation|GetActorLocation))
  (|CallParentFunction)
  (bind _outhit (Collision|LineTraceByChannel _returnvalue (- _returnvalue "0, 0,1000.000000") "TraceTypeQuery1" false (Utilities|Array|MakeArray self) "None")))